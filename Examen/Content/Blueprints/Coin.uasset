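; Coin pickup actor that the player collects by touching it.
; When the player pawn overlaps its box, it adds its Coin value to the ThirdPersonCharacter's coin count, destroys itself and plays a coin sound at its location.
; It then calls ShowCoins on the main HUD's in-game widget to display the coins.
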(event `self.Box.OnComponentBeginOverlap`
  (params (OverlappedComponent :type "PrimitiveComponent Object Reference") (OtherActor :type "Actor Object Reference") (OtherComp :type "PrimitiveComponent Object Reference") (OtherBodyIndex :type Integer) (bFromSweep :type Boolean) (SweepResult :type "HitResult Structure (by ref)"))
  (bind _returnvalue (`GameplayStatics.GetPlayerPawn` 0))
  ;[1 1 1] CollectCoins
  (if (== OtherActor _returnvalue)
    (bind _asthird_person_character (cast `/Game/ThirdPersonBP/Blueprints/ThirdPersonCharacter` _returnvalue))
    (set `/Game/ThirdPersonBP/Blueprints/ThirdPersonCharacter.Coins` (+ (`/Game/ThirdPersonBP/Blueprints/ThirdPersonCharacter.Coins` _asthird_person_character) (`self.coin`)) _asthird_person_character)
    (`self.K2_DestroyActor`)
    (`GameplayStatics.PlaySoundAtLocation` "/Game/Blueprints/Prac2/Sounds/Coin.Coin" (`self.K2_GetActorLocation`) (struct) 1.0 1.0 0.0 null null null)
    (bind _ashud_main_hud (cast `/Game/Blueprints/Prac2/HUD_MainHUD` (`PlayerController.GetHUD` (`GameplayStatics.GetPlayerController` 0))))
    (`/Game/Blueprints/Prac2/HUD_INGAME.ShowCoins` (`/Game/Blueprints/Prac2/HUD_MainHUD.IngameBase` _ashud_main_hud))))

(fn `UserConstructionScript`)