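; Main HUD Blueprint that creates the in-game UI and opens the pause menu.
; On BeginPlay it creates the HUD_INGAME widget, calls ShowLife on it and adds it to the viewport.
; Wrapper functions show, hide and set the text of a ShowText reference, which is not assigned in these graphs.
; PauseGame adds a MenuPausa widget to the player screen and switches input to UI only, without pausing the game itself.
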(event `self.ReceiveBeginPlay`
  ;[1 1 1] CreateWidgets
  (bind _returnvalue (`|CreateWidget` "/Game/Blueprints/Prac2/HUD_INGAME.HUD_INGAME_C" (`GameplayStatics.GetPlayerController` 0)))
  (bind _output_get (set `self.IngameBase` _returnvalue))
  (`/Game/Blueprints/Prac2/HUD_INGAME.ShowLife` _output_get)
  (`UserWidget.AddToViewport` _output_get 0))

(fn `PauseGame`
  (bind _returnvalue (`GameplayStatics.GetPlayerController` 0))
  (bind _returnvalue_2 (`|CreateWidget` "/Game/Blueprints/Prac2/MenuPausa.MenuPausa_C" _returnvalue))
  (`UserWidget.AddToPlayerScreen` _returnvalue_2 0)
  (`WidgetBlueprintLibrary.SetInputMode_UIOnlyEx` _returnvalue _returnvalue_2))

(fn `ShowText_Hide`
  (`/Game/Blueprints/Prac2/WID_ShowText.Hide` (`self.ShowText`)))

(fn `ShowText_SetText`
  (params (NewText :type String))
  (`/Game/Blueprints/Prac2/WID_ShowText.Set_Text` (`self.ShowText`) NewText))

(fn `ShowText_Show`
  (`/Game/Blueprints/Prac2/WID_ShowText.Show` (`self.ShowText`)))

(fn `UserConstructionScript`)